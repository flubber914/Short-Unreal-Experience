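; Alien scanner actor that turns Niagara scan particles into detection events for level actors implementing BPI_LevelEvents.
; It registers as the NSScan export callback and starts with actor collision disabled, using that flag as the scan-active switch.
; When enabled, it sphere-overlaps Vehicle objects at each actor-offset particle position, printing and broadcasting EventScanMessage per hit.
; When disabled, incoming particle data broadcasts NoScanMessage instead.
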(event EventBeginPlay
  (Niagara|SetNiagaraVariable(Object) (Variables|Default|GetNS_Scan) "User.UP_Collide" self)
  (Collision|SetActorEnableCollision self false))

(event EventParticleData
  (params (Data :type Array%20of%20Basic%20Particle%20Data%20Structures) (NiagaraSystem :type Niagara%20System%20Object%20Reference) (SimulationPositionOffset :type Vector%20%28by%20ref%29 :default "0, 0, 0"))
  (bind _outactors (Actor|GetAllActorswithInterface "/Game/Interfaces/BPI_LevelEvents.BPI_LevelEvents_C"))
  (if (Collision|GetActorEnableCollision)
    (for _array_element Data
      (bind _outactors_2 (Collision|SphereOverlapActors (+ (.Position (Utilities|Struct|BreakBasicParticleData _array_element)) (Transformation|GetActorLocation)) 1e+02 (Utilities|Array|MakeArray (Utilities|Enum|LiteralenumEObjectTypeQuery "ObjectTypeQuery5")) 0))
      (bind _array_element_2 (Utilities|Array|ForEachLoopwithBreak _outactors_2)
        (:LoopBody
          (Development|PrintString (Utilities|GetDisplayName _array_element_2))
          (Class|BPILevelEvents|CallEventScan(Message) _outactors))))
    (else
      (Class|BPILevelEvents|CallNoScan(Message) _outactors))))

(fn ConstructionScript)
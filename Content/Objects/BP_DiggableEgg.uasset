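; A diggable egg actor that reveals a buried alien egg with an animated rise and a particle effect.
; Calling FindEgg plays a timeline that moves the egg component's relative location and rotates the whole actor.
; When the timeline finishes, the found-egg Niagara effect, deactivated at BeginPlay, snaps to the egg's world position and activates.
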(event Custom|FindEgg
  (bind _ns_eggfound (Variables|Default|GetNS_EggFound))
  (bind (_direction _location _rotation) (Timeline|EggAnimate Play)
    (:Update
      (Transformation|SetRelativeLocation (Variables|Default|GetBP_AlienEgg) _location false false)
      (Transformation|SetActorRotation (Math|Rotator|MakeRotator 0.0 0.0 _rotation)))
    (:Finished
      (Transformation|SetWorldLocation _ns_eggfound (Transformation|GetWorldLocation (Variables|Default|GetBP_AlienEgg)) false false)
      (Components|Activation|Activate _ns_eggfound false))))

(event EventBeginPlay
  (Components|Activation|Deactivate (Variables|Default|GetNS_EggFound)))

(event Collision|EventActorBeginOverlap
  (params (OtherActor :type Actor%20Object%20Reference)))

(event EventTick
  (params (DeltaSeconds :type Float%20%28single-precision%29)))

(fn ConstructionScript)